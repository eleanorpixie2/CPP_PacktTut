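; BouncingCube_Interact_BP is an interactable physics cube that reacts to being used or shot with motion and floating debug text.
; OnInteract gives the cube, if it is simulating physics, an upward velocity-change impulse scaled by JumpStrength and shows a happy message.
; Point damage applies an impulse at the hit location against the hit normal, scaled by HitStrength, and prints a red complaint.
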(event EventBeginPlay)

(event Collision|EventActorBeginOverlap
  (params (OtherActor :type Actor%20Object%20Reference)))

(event EventTick
  (params (DeltaSeconds :type Float%20%28single-precision%29)))

(event Game|Damage|EventPointDamage
  (params (Damage :type Float%20%28single-precision%29) (DamageType :type Damage%20Type%20Object%20Reference) (HitLocation :type Vector :default "0, 0, 0") (HitNormal :type Vector :default "0, 0, 0") (HitComponent :type Primitive%20Component%20Object%20Reference) (BoneName :type Name :default "None") (ShotFromDirection :type Vector :default "0, 0, 0") (InstigatedBy :type Controller%20Object%20Reference) (DamageCauser :type Actor%20Object%20Reference) (HitInfo :type Hit%20Result%20Structure%20%28by%20ref%29))
  (Physics|AddImpulseatLocation (Variables|Default|GetCube) (* HitNormal (* -1 (Variables|Default|GetHitStrength))) HitLocation "None")
  (Rendering|Debug|DrawDebugString (Transformation|GetActorLocation) "Ow, Stop it" 0 "(R=1.000000,G=0.000000,B=0.000000,A=1.000000)" 2.5))

(event EventOnInteract
  (params (Interactor :type Actor%20Object%20Reference))
  (if (Physics|IsSimulatingPhysics (Variables|Default|GetCube) "None")
    (Physics|AddImpulse (Variables|Default|GetCube) (* "0, 0,1.000000" (Variables|Default|GetJumpStrength)) "None" true)
    (Rendering|Debug|DrawDebugString (Transformation|GetActorLocation) "I'm happy to see you!" 0 "(R=0.149924,G=0.026801,B=0.395833,A=1.000000)" 2.5)))

(fn ConstructionScript)